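; AK rifle Blueprint that handles hitscan firing and ammo for the CloudRobot player character.
; Fire spends a round and line-traces from the player's camera, showing a hitmarker widget on AI hits, reducing their health and destroying them at zero.
; Reload sets the clip from reserve ammo, discarding any rounds left in it.
; Disconnected leftover nodes hold a projectile spawn and a debug trace.
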(event `Fire`
  (set `self.Ammo` (- (`self.Ammo`) 1))
  (bind _ascloud_robot (cast `/Game/RawContent/CloudRobot` (`GameplayStatics.GetPlayerCharacter` 0)))
  (bind _camera (`/Game/RawContent/CloudRobot.Camera` _ascloud_robot))
  (bind _returnvalue (`SceneComponent.K2_GetComponentLocation` _camera))
  (bind _outhit (`KismetSystemLibrary.LineTraceSingle` _returnvalue (+ _returnvalue (* (`KismetMathLibrary.GetForwardVector` (`SceneComponent.K2_GetComponentRotation` _camera)) 3000.0)) "TraceTypeQuery1"))
  (bind _asai (cast `/Game/RawContent/AI/AIChar/AI` (`.HitActor` (`GameplayStatics.BreakHitResult` _outhit))))
  (bind _returnvalue_2 (`|CreateWidget` "/Game/RawContent/Objects/AK/HitmarkerHUD.HitmarkerHUD_C"))
  (`UserWidget.AddToViewport` _returnvalue_2 0)
  (bind _output_get (set `/Game/RawContent/AI/AIChar/AI.HealthAI` (- (`/Game/RawContent/AI/AIChar/AI.HealthAI` _asai) 0.2) _asai))
  (if (<= _output_get 0.0)
    (`self.K2_DestroyActor` _asai)))

(fn `Reload`
  (if (== (`self.Ammo`) (`self.ClipSize`))
    _
    (elif (> (`self.MaxAmmo`) (`self.ClipSize`))
      (set `self.Ammo` (`self.ClipSize`))
      (set `self.MaxAmmo` (- (`self.MaxAmmo`) (`self.ClipSize`)))
      (else
        (set `self.Ammo` (`self.MaxAmmo`))
        (set `self.MaxAmmo` 0)))))

(fn `UserConstructionScript`)